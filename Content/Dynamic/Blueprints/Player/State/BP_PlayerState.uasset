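; Player state for the Harvest game mode that holds a player's Water, Seeds and Plants resources.
; On the authority, it registers ServerTick with GM_Harvest, which drives passive water gain at WaterRate, clamped between zero and MaxWater.
; Each new water value is sent through an RPC.
; The RPC events for all three resources store the received value and call the matching updated notification.
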(event Custom|ServerTick
  (params (deltaTime :type Float%20%28double-precision%29))
  (CallFunction|PassiveWaterGain deltaTime))

(event Custom|RPC_UpdateWater
  (params (newWaterValue :type Float%20%28double-precision%29))
  (bind _output_get (Variables|Parameters|Setwater newWaterValue))
  (Default|CallOnWaterUpdated _output_get))

(event Custom|RPC_UpdatePlantsValue
  (params (newSeedsValue :type Integer))
  (bind _output_get (Variables|Parameters|Setplants newSeedsValue))
  (Default|CallOnPlantsUpdated _output_get))

(event Custom|RPC_UpdateSeeds
  (params (newSeedsValue :type Integer))
  (bind _output_get (Variables|Parameters|Setseeds newSeedsValue))
  (Default|CallOnSeedsUpdated _output_get))

(event EventBeginPlay
  (Networking|SwitchHasAuthority
    (:Authority
      (bind _asgm_harvest (Utilities|Casting|CastToGM_Harvest (Game|GetGameMode)))
      (EventDispatchers|AssignOnServerTick _asgm_harvest (delegate Custom|ServerTick)))))

(event EventTick
  (params (DeltaSeconds :type Float%20%28single-precision%29)))

(fn ConstructionScript)

(fn PassiveWaterGain
  (params (deltaTime :type Float%20%28double-precision%29))
  (bind _output_get (Variables|Parameters|Setwater (Math|Float|Clamp(Float) (+ (Variables|Parameters|Getwater) (* deltaTime (Variables|Parameters|GetwaterRate))) 0.0 (Variables|Parameters|GetmaxWater))))
  (CallFunction|RPCUpdateWater _output_get))