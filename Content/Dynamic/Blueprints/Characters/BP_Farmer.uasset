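; BP_Farmer is a farmer character that registers with GM_Harvest on BeginPlay and carries out tasks requested of it.
; RequestTask walks it to a target location, sets the current task on arrival, then resets that task after the given duration.
; The latent MoveTo macro loops each tick via DelayUntilNextTick, adding horizontal movement input and optionally turning the capsule toward the target until within tolerance.
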(event Custom|RequestTask
  (params (taskType :type ETaskType%20Enum :default "NewEnumerator4") (taskTime :type Float%20%28double-precision%29) (targetLocation :type Vector))
  (Utilities|Moveto true targetLocation 5e+01
    (:Completed
      (Variables|Default|SetcurrentTask taskType)
      (Utilities|FlowControl|Delay taskTime)
      (Variables|Default|SetcurrentTask "NewEnumerator4"))))

(event EventBeginPlay
  (bind _asgm_harvest (Utilities|Casting|CastToGM_Harvest (Game|GetGameMode)))
  (Default|AddFarmer _asgm_harvest self))

(event EventTick
  (params (DeltaSeconds :type Float%20%28single-precision%29)))

(fn ConstructionScript)