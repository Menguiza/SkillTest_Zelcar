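; Game mode for Harvest that builds the world as a grid of plot actors on BeginPlay.
; BuildWorld loops over rows and columns, offsetting each plot along the origin component's forward and right vectors, or from world zero if the origin is invalid.
; Each plot is spawned scaled to the plot dimensions, attached to the game mode and added to AvailablePlots.
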(event EventBeginPlay
  (CallFunction|BuildWorld (Variables|Default|GetDefaultSceneRoot) (Variables|Parameters|GetworldDimensions) "(X=100.000000,Y=100.000000)"))

(event EventTick
  (params (DeltaSeconds :type Float%20%28single-precision%29)))

(fn ConstructionScript)

(fn BuildWorld
  (params (origin :type Scene%20Component%20Object%20Reference) (gridDimensions :type Vector%202D%20Structure) (plotDimensions :type Vector%202D%20Structure :default "(X=100.000000,Y=100.000000)"))
  (bind (_x _y) (Math|Vector2D|BreakVector2D gridDimensions))
  (bind _returnvalue (Math|Transform|MakeTransform "0, 0, 0"))
  (bind _returnvalue_2 (Utilities|IsValid origin))
  (bind _returnvalue_3 (Transformation|GetWorldTransform origin))
  (bind _returnvalue_4 (/ plotDimensions "(X=100.000000,Y=100.000000)"))
  (bind _returnvalue_5 (select _returnvalue_2 _returnvalue_3 _returnvalue))
  (bind (_location _rotation) (Math|Transform|BreakTransform _returnvalue_5))
  ;[1 1 1] Proccess Grid Dimensions
  (bind _output_get (LocalVariables|Setcolumns (Math|Integer|Max(Integer) (- (Math|Float|Floor _x) 1))))
  (bind _output_get_2 (LocalVariables|Setrows (Math|Integer|Max(Integer) (- (Math|Float|Floor _y) 1))))
  (for _index (range 0 _output_get_2)
    (for _index_2 (range 0 _output_get)
      ;[1 1 1] Spawn Plot
      (bind _returnvalue_6 (Game|SpawnActorfromClass (Variables|References|GetplotClass) (Math|Transform|MakeTransform (+ (* (Math|Vector|Normalize (Math|Vector|GetForwardVector _rotation)) (* _index (.y plotDimensions))) (* (Math|Vector|Normalize (Math|Vector|GetRightVector _rotation)) (* _index_2 (.x plotDimensions))) _location) _rotation (Math|Vector|MakeVector (.x _returnvalue_4) (.y _returnvalue_4) 1.0)) "Undefined" "MultiplyWithRoot" 0 0))
      (Transformation|AttachActorToActor _returnvalue_6 self "None" "KeepWorld" "KeepWorld" "KeepWorld" true)
      (Utilities|Array|Add (Variables|Utility|GetavailablePlots) _returnvalue_6))))